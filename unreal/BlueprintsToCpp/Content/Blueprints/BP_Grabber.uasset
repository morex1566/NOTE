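; BP_Grabber is a component that lets its owner pick up, hold and release physics objects through a physics handle.
; Grab sphere-traces for physics bodies, enables simulation on the hit component and grabs it at its center of mass.
; Tick moves the held target to the hold location with the grabber's rotation.
; A successful grab also calls Pickup on the actor's BP_QuestTriggerPickup component, if present.
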(event EventBeginPlay)

(event EventTick
  (params (DeltaSeconds :type Float%20%28single-precision%29))
  (Class|PhysicsHandleComponent|SetTargetLocationandRotation (Class|Grabber|GetPhysicsComponent) (Class|Grabber|GetHoldLocation) (Transformation|GetWorldRotation)))

(event EventNotifyQuestActor
  (params (actor :type Actor%20Object%20Reference))
  (bind _returnvalue (Actor|GetComponentbyClass actor "/Game/Quests/CompletionTriggers/BP_QuestTriggerPickup.BP_QuestTriggerPickup_C"))
  (Utilities|IsValid _returnvalue
    (:Is%20Valid
      (Default|Pickup _returnvalue))))

(fn Grab
  (bind (_actor _primitivecomponent _returnvalue) (CallFunction|TraceforPhysicsBodies))
  (if _returnvalue
    (Physics|SetSimulatePhysics _primitivecomponent true) ; Some actors may not yet.
    (Physics|Components|PhysicsHandle|GrabComponentatLocationwithRotation (Class|Grabber|GetPhysicsComponent) _primitivecomponent "None" (Physics|GetCenterOfMass _primitivecomponent "None") "0, 0, 0")
    (CallFunction|NotifyQuestActor _actor)))

(fn Release
  (Physics|Components|PhysicsHandle|ReleaseComponent (Class|Grabber|GetPhysicsComponent)))

(fn TraceforPhysicsBodies
  (bind (_outhit _returnvalue) (Collision|SphereTraceForObjects (Transformation|GetWorldLocation) (Class|Grabber|GetMaxGrabLocation) (Variables|Default|GetGrabRadius) (Utilities|Array|MakeArray "ObjectTypeQuery4") false 0 "None"))
  (return (.HitActor (Collision|BreakHitResult _outhit)) (.HitComponent (Collision|BreakHitResult _outhit)) _returnvalue))